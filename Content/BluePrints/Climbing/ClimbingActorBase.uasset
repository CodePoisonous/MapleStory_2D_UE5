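; ClimbingActorBase is a base actor for climbable objects that tells players when they can climb.
; On the server, overlapping Box sends a CanClimb message to actors tagged "player", passing itself as the climb object, and leaving withdraws it.
; UpperBox disables upward climbing while the player overlaps it and re-enables it on exit, apparently marking the top limit.
; Player references are fetched through message calls on the overlapping actor.
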(event OnComponentBeginOverlap(Box)
  (params (OverlappedComponent :type Primitive%20Component%20Object%20Reference) (OtherActor :type Actor%20Object%20Reference) (OtherComp :type Primitive%20Component%20Object%20Reference) (OtherBodyIndex :type Integer) (bFromSweep :type Boolean) (SweepResult :type Hit%20Result%20Structure%20%28by%20ref%29))
  (Networking|SwitchHasAuthority
    (:Authority
      (if (Actor|ActorHasTag OtherActor "player")
        (bind _player (Class|INTPlayerBase|GetPlayerRef(Message) OtherActor))
        (Default|CanClimb _player true self)))))

(event OnComponentEndOverlap(Box)
  (params (OverlappedComponent :type Primitive%20Component%20Object%20Reference) (OtherActor :type Actor%20Object%20Reference) (OtherComp :type Primitive%20Component%20Object%20Reference) (OtherBodyIndex :type Integer))
  (Networking|SwitchHasAuthority
    (:Authority
      (if (Actor|ActorHasTag OtherActor "player")
        (bind _player (Class|INTPlayerBase|GetPlayerRef(Message) OtherActor))
        (Default|CanClimb _player false self)))))

(event OnComponentBeginOverlap(UpperBox)
  (params (OverlappedComponent :type Primitive%20Component%20Object%20Reference) (OtherActor :type Actor%20Object%20Reference) (OtherComp :type Primitive%20Component%20Object%20Reference) (OtherBodyIndex :type Integer) (bFromSweep :type Boolean) (SweepResult :type Hit%20Result%20Structure%20%28by%20ref%29))
  (Networking|SwitchHasAuthority
    (:Authority
      (if (Actor|ActorHasTag OtherActor "player")
        (bind _player (Class|INTPlayerBase|GetPlayerRef(Message) OtherActor))
        (Class|INTPlayerBase|SetCanClimbUp(Message) _player false)))))

(event OnComponentEndOverlap(UpperBox)
  (params (OverlappedComponent :type Primitive%20Component%20Object%20Reference) (OtherActor :type Actor%20Object%20Reference) (OtherComp :type Primitive%20Component%20Object%20Reference) (OtherBodyIndex :type Integer))
  (Networking|SwitchHasAuthority
    (:Authority
      (if (Actor|ActorHasTag OtherActor "player")
        (bind _player (Class|INTPlayerBase|GetPlayerRef(Message) OtherActor))
        (Class|INTPlayerBase|SetCanClimbUp(Message) _player true)))))

(fn ConstructionScript)