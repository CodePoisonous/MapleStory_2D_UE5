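; Player controller that manages a player's UI, character selection and pawn spawning.
; On BeginPlay, client-prefixed events show the character selection widget and create the main HUD widget, which later receives health updates.
; Selection passes through a server-prefixed event to the GameMode via a message call to request a spawn.
; SpawnPlayer then spawns and possesses the chosen character.
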(event Custom|CL_UpdateHealthValue
  (params (Percent :type Float%20%28single-precision%29))
  (Default|UpdateHealth (Variables|Default|GetWB_Main) Percent))

(event Custom|CL_InitializeWidgets
  ;[1 1 1] UI管理
  (bind _returnvalue (UserInterface|CreateWidget "/Game/BluePrints/UI/WB_CharactorSelection.WB_CharactorSelection_C")) ; 选择角色UI
  (bind _output_get (Variables|Default|SetWB_CharactorSelection _returnvalue))
  (UserInterface|Viewport|AddtoViewport _output_get 0)
  (bind _returnvalue_2 (UserInterface|CreateWidget "/Game/BluePrints/UI/WB_Main.WB_Main_C")) ; 主界面UI
  (Variables|Default|SetWB_Main _returnvalue_2))

(event Custom|SRV_SelectCharactor
  (params (Player :type Actor%20Class%20Reference) (SpawnLocation :type Vector))
  ;[1 1 1] 角色创建管理
  (bind _mygamemode (Class|INTGameMode|GetGameModeRef(Message) (Game|GetGameMode)))
  (Class|INTGameMode|RequestSpawnPlayer(Message) _mygamemode self Player SpawnLocation))

(event EventSpawnPlayer
  (params (Player :type Actor%20Class%20Reference) (SpawnTransform :type Transform))
  ;[1 1 1] 角色创建管理
  (bind _returnvalue (Game|SpawnActorfromClass Player SpawnTransform "AdjustIfPossibleButAlwaysSpawn" "MultiplyWithRoot" 0 0))
  (bind _player (Class|INTPlayerBase|GetPlayerRef(Message) _returnvalue))
  (Pawn|Possess _player))

(event EventUpdateHealthValue
  (params (Percent :type Float%20%28double-precision%29))
  (CallFunction|CLUpdateHealthValue Percent))

(event EventBeginPlay
  ;[1 1 1] UI管理
  (CallFunction|InitializeWidgets))

(event EventInitializeWidgets
  ;[1 1 1] UI管理
  (CallFunction|CLInitializeWidgets))

(event EventSelectCharactor
  (params (Player :type Actor%20Class%20Reference) (SpawnLocation :type Vector :default "0, 0, 0"))
  ;[1 1 1] 角色创建管理
  (CallFunction|SRVSelectCharactor Player SpawnLocation))

(fn ConstructionScript)

(fn GetMyPlayerControllerRef
  (return self))