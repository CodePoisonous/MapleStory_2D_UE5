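; TM_DragonRoad is a tilemap Blueprint that pauses the player camera while a player is inside either of its two side trigger boxes.
; LeftBox and RightBox overlap events run only on the server and filter for actors tagged "Player".
; Begin overlap gets the player reference through GetPlayerRefMessage and calls PausePlayerCamerA with true; end overlap calls it with false.
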(event OnComponentBeginOverlap(LeftBox)
  (params (OverlappedComponent :type Primitive%20Component%20Object%20Reference) (OtherActor :type Actor%20Object%20Reference) (OtherComp :type Primitive%20Component%20Object%20Reference) (OtherBodyIndex :type Integer) (bFromSweep :type Boolean) (SweepResult :type Hit%20Result%20Structure%20%28by%20ref%29))
  ;[1 1 1] 开始重叠
  (Networking|SwitchHasAuthority ; 保证重叠响应在服务器端
    (:Authority
      (if (Actor|ActorHasTag OtherActor "Player")
        (bind _player (Class|INTPlayerBase|GetPlayerRef(Message) OtherActor))
        (Default|PausePlayerCamerA _player true)))))

(event OnComponentBeginOverlap(RightBox)
  (params (OverlappedComponent :type Primitive%20Component%20Object%20Reference) (OtherActor :type Actor%20Object%20Reference) (OtherComp :type Primitive%20Component%20Object%20Reference) (OtherBodyIndex :type Integer) (bFromSweep :type Boolean) (SweepResult :type Hit%20Result%20Structure%20%28by%20ref%29))
  ;[1 1 1] 开始重叠
  (Networking|SwitchHasAuthority
    (:Authority
      (if (Actor|ActorHasTag OtherActor "Player")
        (bind _player (Class|INTPlayerBase|GetPlayerRef(Message) OtherActor))
        (Default|PausePlayerCamerA _player true)))))

(event OnComponentEndOverlap(LeftBox)
  (params (OverlappedComponent :type Primitive%20Component%20Object%20Reference) (OtherActor :type Actor%20Object%20Reference) (OtherComp :type Primitive%20Component%20Object%20Reference) (OtherBodyIndex :type Integer))
  ;[1 1 1] 结束重叠
  (Networking|SwitchHasAuthority
    (:Authority
      (if (Actor|ActorHasTag OtherActor "Player")
        (bind _player (Class|INTPlayerBase|GetPlayerRef(Message) OtherActor))
        (Default|PausePlayerCamerA _player false)))))

(event OnComponentEndOverlap(RightBox)
  (params (OverlappedComponent :type Primitive%20Component%20Object%20Reference) (OtherActor :type Actor%20Object%20Reference) (OtherComp :type Primitive%20Component%20Object%20Reference) (OtherBodyIndex :type Integer))
  ;[1 1 1] 结束重叠
  (Networking|SwitchHasAuthority
    (:Authority
      (if (Actor|ActorHasTag OtherActor "Player")
        (bind _player (Class|INTPlayerBase|GetPlayerRef(Message) OtherActor))
        (Default|PausePlayerCamerA _player false)))))

(fn ConstructionScript)