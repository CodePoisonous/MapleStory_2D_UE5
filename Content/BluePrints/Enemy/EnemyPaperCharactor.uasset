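; Paper2D enemy character Blueprint that swaps its flipbook between idle and move animations based on a replicated movement state.
; SetMovementState forwards to SRV_SetMovementState, which writes m_IsMoving.
; The variable's OnRep then applies the matching flipbook from AnimalInfo to the sprite.
; GetEnemyRef returns the actor itself.
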(event Custom|SRV_SetMovementState
  (params (IsMoving :type Boolean))
  (Variables|Default|Setm_IsMoving IsMoving))

(event EventSetMovementState
  (params (IsMoving :type Boolean))
  (CallFunction|SRVSetMovementState IsMoving))

(fn ConstructionScript
  (|CallParentFunction))

(fn OnRepMIsMoving
  (bind _sprite (Variables|Default|GetSprite))
  (bind _animalinfo (Variables|Default|GetAnimalInfo))
  (bind (_idleanimation _moveanimation) (Utilities|Struct|BreakST_EnemyInfo _animalinfo))
  (if (not (Variables|Default|Getm_IsMoving))
    (Sprite|SetFlipbook _sprite _idleanimation)
    (else
      (Sprite|SetFlipbook _sprite _moveanimation))))

(fn GetEnemyRef
  (return self))