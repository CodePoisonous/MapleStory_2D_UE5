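; Networked Paper2D player character for a side-scrolling game, handling run and jump input, spawn placement and its own follow camera.
; Server events set spawn location and movement state; RepNotifies move the actor and switch or flip the flipbook.
; Jump sounds go through a server-to-multicast event.
; A spawned BP_Camera lerps toward a timer-sampled player location via a repeatedly restarted timeline; pausing that sampling halts following at map edges.
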(event Custom|SetPlayerSpawnLocation
  ;[1 1 1] 初始化玩家位置
  (CallFunction|SRVSetPlayerSpawnLocation))

(event Custom|SRV_SetMovementState
  (params (m_MovementState :type E_MovementState%20Enum :default "NewEnumerator0"))
  ;[1 1 1] 移动状态事件响应
  (Variables|Default|Setm_MovementState m_MovementState))

(event Custom|SRV_SetPlayerSpawnLocation
  ;[1 1 1] 初始化玩家位置
  (bind _mygamemode (Class|INTGameMode|GetGameModeRef(Message) (Game|GetGameMode)))
  (Variables|Default|Setm_Player%20Spawn%20Location (Variables|/Game/BluePrints/MyGameMode.MyGameMode_C|GetPlayerSpawnLocation _mygamemode)))

(event Custom|SRV_MC_Jump
  (params (Sound :type Sound%20Base%20Object%20Reference) (Location :type Vector))
  ;[1 1 1] 声音状态事件响应
  (CallFunction|MCJump Sound Location))

(event Custom|MC_Jump
  (params (Sound :type Sound%20Base%20Object%20Reference) (Location :type Vector))
  ;[1 1 1] 声音状态事件响应
  (Audio|PlaySoundatLocation Sound Location "0, 0, 0" 1.0 1.0 0.0 0 0 0 0))

(event Custom|UpdatePlayerCameraPosition
  ;[1 1 1] 更新摄像机的平滑移动
  ;;[1 1 1] 设置摄像机跟随角色
  (bind _movementalpha (Timeline|PlayerCameraPosition PlayFromStart)
    (:Update
      (bind _m_playercamera (Variables|Default|Getm_PlayerCamera)
        (:then
          (Transformation|SetActorLocation _m_playercamera (Math|Vector|Lerp(Vector) (Transformation|GetActorLocation (Variables|Default|Getm_PlayerCamera)) (Variables|Default|Getm_CurrentPlayerLocation) _movementalpha) false false))
        (:else)))))

(event Custom|CL_PausePlayerCamera
  (params (IsPause :type Boolean))
  (bind _m_getcurrentlocationhandle (Variables|Default|Getm_GetCurrentLocationHandle))
  ;[1 1 1] 更新摄像机的平滑移动
  ;;[1 1 1] 摄像机边界暂停移动
  (if IsPause
    (Utilities|Time|PauseTimerbyHandle _m_getcurrentlocationhandle)
    (else
      (Utilities|Time|UnpauseTimerbyHandle _m_getcurrentlocationhandle))))

(event EventSetMovementState
  (params (MoveState :type E_MovementState%20Enum :default "NewEnumerator0"))
  ;[1 1 1] 移动状态事件响应
  (CallFunction|SRVSetMovementState MoveState))

(event EventBeginPlay
  ;[1 1 1] 初始化玩家位置
  (CallFunction|SetPlayerSpawnLocation)
  (Utilities|FlowControl|Delay 0.0001) ; 需等待角色生成，否则后续的摄像机找不到角色
  (bind _returnvalue (Game|SpawnActorfromClass "/Game/BluePrints/BP_Camera.BP_Camera_C" (Math|Transform|MakeTransform (Transformation|GetActorLocation)) "AdjustIfPossibleButAlwaysSpawn" "MultiplyWithRoot" 0 0))
  (Variables|Default|Setm_PlayerCamera _returnvalue)
  (bind _myplayercotroller (Class|INTPlayerController|GetMyPlayerControllerRef(Message) (Pawn|GetController)))
  (Utilities|IsValid _myplayercotroller
    (:Is%20Valid
      (Game|Player|SetViewTargetwithBlend _myplayercotroller (Variables|Default|Getm_PlayerCamera) 0.0 "VTBlend_Linear" 0.0 false)
      ;[1 1 1] 更新摄像机的平滑移动
      ;;[1 1 1] 设置摄像机跟随角色
      (bind _returnvalue_2 (Utilities|Time|SetTimerbyEvent (delegate Custom|UpdatePlayerCameraPosition) 0.03 true)) ; 定时循环触发事件，以节约资源
      (Variables|Default|Setm_UpdatePlayerCameraHandle _returnvalue_2) ; 定时器id号
      (bind _returnvalue_3 (Utilities|Time|SetTimerbyFunctionName 0 "GetCurrentPlayerLocation" 0.1 true)) ; 设置这个定时器的目的是为了让角色到达地图边缘时，相机以非常慢的速度更新位置
      (Variables|Default|Setm_GetCurrentLocationHandle _returnvalue_3))))

(event EventPausePlayerCamerA
  (params (pause :type Boolean))
  ;[1 1 1] 更新摄像机的平滑移动
  ;;[1 1 1] 摄像机边界暂停移动
  (CallFunction|CLPausePlayerCamera pause))

(event Input|ActionEvents|InputActionJump
  (params (Key :type Key%20Structure))
  ;[1 1 1] 玩家跳跃
  (:Pressed
    (if (CallFunction|IsNotJumping)
      (Character|Jump)
      (CallFunction|SRVMCJump (Utilities|Struct|BreakST_PlayerSoundInfo (Variables|Default|Getm_PlayerSoundInfo)) (Transformation|GetActorLocation)))))

(event Input|AxisEvents|InputAxisMove_Left_Right
  (params (AxisValue :type Float%20%28single-precision%29))
  ;[1 1 1] 玩家移动
  (Pawn|Input|AddMovementInput (Math|Vector|GetForwardVector (Pawn|GetControlRotation :!class /Script/Engine.Pawn)) AxisValue false)
  (if (AI|Components|NavMovement|IsFalling (Variables|Character|GetCharacterMovement))
    (if (> (.Z (Math|Vector|BreakVector (Transformation|GetVelocity))) 0.0) ; 跳跃/下坠
      (CallFunction|SetMovementState "NewEnumerator3")
      (else
        (CallFunction|SetMovementState "NewEnumerator4")))
    (elif (== AxisValue 0.0) ; 移动/待机
      (CallFunction|SetMovementState "NewEnumerator0")
      (elif (> AxisValue 0.0) ; 左/右移
        (CallFunction|SetMovementState "NewEnumerator2")
        (else
          (CallFunction|SetMovementState "NewEnumerator1"))))))

(fn ConstructionScript
  (|CallParentFunction))

(fn IsNotJumping
  (return (not (AI|Components|NavMovement|IsFalling (Variables|Character|GetCharacterMovement)))))

(fn OnRepMMovementState
  (bind _m_playeraniminfo (Variables|Default|Getm_PlayerAnimInfo))
  (bind (_idleanim _runanim _jumpanim _fallanim) (Utilities|Struct|BreakST_PlayerAnimInfo _m_playeraniminfo))
  (switch Utilities|FlowControl|Switch|SwitchonE_MovementState (Variables|Default|Getm_MovementState)
    (:NewEnumerator0
      (Sprite|SetFlipbook (Variables|Default|GetSprite) _idleanim))
    (:NewEnumerator1
      (Transformation|SetRelativeRotation (Variables|Default|GetSprite) "0.000000,-180.000000,0.000000" false false)
      (Sprite|SetFlipbook (Variables|Default|GetSprite) _runanim))
    (:NewEnumerator2
      (Transformation|SetRelativeRotation (Variables|Default|GetSprite) "0, 0, 0" false false)
      (Sprite|SetFlipbook (Variables|Default|GetSprite) _runanim))
    (:NewEnumerator3
      (Sprite|SetFlipbook (Variables|Default|GetSprite) _jumpanim))
    (:NewEnumerator4
      (Sprite|SetFlipbook (Variables|Default|GetSprite) _fallanim))))

(fn OnRepMPlayerSpawnLocation
  (Transformation|SetActorLocation (Variables|Default|Getm_Player%20Spawn%20Location) false false))

(fn GetCurrentPlayerLocation
  (Variables|Default|Setm_CurrentPlayerLocation (Transformation|GetActorLocation)))

(fn GetPlayerRef
  (return self))